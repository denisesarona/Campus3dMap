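; Shared helper functions for a building-information feature that uses a local MySQL database.
; DatabaseConnection opens the hard-coded capstonedb link, and DatabaseQueryArrayElement runs a query, returning a field value and index from inside its row loop.
; Other helpers pack building fields into SBuildingInfo, spawn WB_BldgInfo child widgets and switch widget-switcher pages.
; LoadURLtoWebBrowser adds a WB_WebBrowser to the viewport without using its ID input.
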(fn `CreateTextWidget`
  (params (Target :type "PanelWidget Object Reference") (BuildingName :type Text) (DeptID :type Text) (DepartmentName :type Text) (Description :type Text) (`Key Features` :type Text) (AmenitiesName :type Text) (NumFloors :type Text))
  ;[1 1 1] Create Text Widget
  (bind _returnvalue (`|CreateWidget` "/Game/Widgets/WB_BldgInfo.WB_BldgInfo_C" null (make `/Game/DataAssets/S_BuildingInfo` BuildingName DeptID DepartmentName Description `Key Features` AmenitiesName NumFloors)))
  (`PanelWidget.AddChild` Target _returnvalue))

(fn `DatabaseConnection`
  (returns (Connection :type "MySQLConnection Object Reference"))
  ;[1 1 1] Database connection
  (bind _connection (`/MySQLConnectorUE4Plugin/Blueprints/Macros/SQLDatabaseMacros.MySQL_Connect` "localhost" "root" "" "capstonedb")
    (:`Success`
      (return _connection))))

(fn `DatabaseQueryArrayElement`
  (params (Query :type String) (Connection :type "MySQLConnection Object Reference"))
  (returns (`Array Element Value` :type String) (`Array Index` :type Integer))
  ;[1 1 1] Database Query Accessing each Specific Array Element
  (bind _returnvalue (`MySQLDatabase.MySQLConnectorGetData` Query Connection))
  (for _array_element (`.ResultRows` (break `MySQLConnectoreQueryResult` _returnvalue))
    (for (_array_element_2 _array_index) (`.Fields` (break `MySQLConnectorQueryResultRow` _array_element))
      (return (`.Value` (break `MySQLConnectorKeyValuePair` _array_element_2)) _array_index))))

(fn `LoadURLtoWebBrowser`
  (params (ID :type Text))
  (bind _returnvalue (`|CreateWidget` "/Game/Widgets/WB_WebBrowser.WB_WebBrowser_C"))
  (`UserWidget.AddToViewport` _returnvalue 0))

(fn `RetrieveBuildingStruct`
  (params (BuildingName :type Text) (DeptID :type Text) (DepartmentName :type Text) (Description :type Text) (`Key Features` :type Text) (AmenitiesName :type Text) (NumFloors :type Text))
  (returns (OutputBuildingName :type Text) (OutputDeptID :type Text) (OutputDepartmentName :type Text) (OutputDescription :type Text) (`OutputKey Features` :type Text) (OutputAmenitiesName :type Text) (OutputNumFloors :type Text))
  (bind (_buildingname _deptid _departmentname _description _keyfeatures _amenitiesname _numfloors) (break `/Game/DataAssets/S_BuildingInfo` (make `/Game/DataAssets/S_BuildingInfo` BuildingName DeptID DepartmentName Description `Key Features` AmenitiesName NumFloors)))
  ;[1 1 1] Retrieve Building Information Structure
  (return _buildingname _deptid _departmentname _description _keyfeatures _amenitiesname _numfloors))

(fn `SetActiveWidget`
  (params (Target :type "WidgetSwitcher Object Reference") (Index :type Integer))
  (locals (AlreadyVisible :type Boolean))
  ;[1 1 1] Set Active Widget in Widget Switcher
  (if (not (`local.AlreadyVisible`))
    (`WidgetSwitcher.SetActiveWidgetIndex` Target Index)
    (return)
    (else
      (`KismetSystemLibrary.PrintString` null "Data already displayed"))))